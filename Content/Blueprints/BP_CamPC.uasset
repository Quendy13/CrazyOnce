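; BP_CamPC is an interactable computer that lets the player view the level's BP_SecurityCam actors.
; On BeginPlay it caches all cameras in the level.
; Interact toggles viewing: it moves input from the character to this actor, ignores look input, and sets the view target to the current camera.
; Space cycles cameras with wrap-around, and Backspace or another Interact restores the player's view and controls.
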(event `self.ReceiveBeginPlay`
  (bind _outactors (`GameplayStatics.GetAllActorsOfClass` "/Game/Blueprints/BP_SecurityCam.BP_SecurityCam_C"))
  (set `self.SecurityCamsRef` _outactors))

(event `/Game/Blueprints/Interfaces/BPI_Interact.Interact`
  (bind _returnvalue (`GameplayStatics.GetPlayerController` 0))
  (if (`self.bIsCamOnline`)
    (`self.EndViewingCam`)
    (else
      (set `self.bIsCamOnline` true)
      (`self.DisableInput` (`GameplayStatics.GetPlayerCharacter` 0) _returnvalue)
      (`Controller.SetIgnoreLookInput` _returnvalue true)
      (`self.EnableInput` _returnvalue)
      (`self.ViewFromCam`))))

(event `EndViewingCam`
  (bind _returnvalue (`GameplayStatics.GetPlayerController` 0))
  (bind _returnvalue_2 (`GameplayStatics.GetPlayerCharacter` 0))
  (set `self.bIsCamOnline` false)
  (`self.DisableInput` _returnvalue)
  (`Controller.ResetIgnoreLookInput` _returnvalue)
  (`self.EnableInput` _returnvalue_2 _returnvalue)
  (`PlayerController.SetViewTargetWithBlend` _returnvalue _returnvalue_2 0.0 "VTBlend_Linear" 0.0 false))

(event `Key|SpaceBar`
  (params (Key :type "Key Structure"))
  (bind _returnvalue (+ (`self.CamIndex`) 1))
  (:`Pressed`
    (set `self.CamIndex` (select `bool` (> _returnvalue (- (`KismetArrayLibrary.Array_Length` (`self.SecurityCamsRef`)) 1)) :`false` _returnvalue))
    (`self.ViewFromCam`)))

(event `Key|BackSpace`
  (params (Key :type "Key Structure"))
  (:`Pressed`
    (`self.EndViewingCam`)))

(fn `UserConstructionScript`)

(fn `ViewFromCam`
  (`PlayerController.SetViewTargetWithBlend` (`GameplayStatics.GetPlayerController` 0) (`|GetArrayItem` (`self.SecurityCamsRef`) (`self.CamIndex`)) 0.0 "VTBlend_Linear" 0.0 false)
  (return))