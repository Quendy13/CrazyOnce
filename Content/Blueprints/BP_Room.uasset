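; BP_Room is a room trigger volume that can start an anomaly event when the first-person character walks in.
; On overlap it sends its room type to the character, then rolls EventProbability unless the game mode is already searching for an anomaly.
; A hit sets that game-mode flag and picks a random room type, flagging matching rooms and calling VisibleThroughCam on their monster spawn points with a whoosh sound.
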(event `self.ReceiveTick`
  (params (DeltaSeconds :type "Float (single-precision)")))

(event `self.ReceiveBeginPlay`
  (bind _asbp_first_person_game_mode (cast `/Game/FirstPerson/Blueprints/BP_FirstPersonGameMode` (`GameplayStatics.GetGameMode`)))
  (set `self.GameModeRef` _asbp_first_person_game_mode)
  (bind _outactors (`GameplayStatics.GetAllActorsOfClass` "BP_Room_C"))
  (set `self.RoomsRef` _outactors))

(event `self.Room.OnComponentBeginOverlap`
  (params (OverlappedComponent :type "PrimitiveComponent Object Reference") (OtherActor :type "Actor Object Reference") (OtherComp :type "PrimitiveComponent Object Reference") (OtherBodyIndex :type Integer) (bFromSweep :type Boolean) (SweepResult :type "HitResult Structure (by ref)"))
  (bind _asbp_first_person_character (cast `/Game/FirstPerson/Blueprints/BP_FirstPersonCharacter` OtherActor))
  (message `/Game/Blueprints/Interfaces/BPI_Interact.EnterRoom` _asbp_first_person_character (`self.RoomType`))
  (if (and (<= (`KismetMathLibrary.RandomFloatInRange` 0.0 1.0) (`self.EventProbability`)) (not (`/Game/FirstPerson/Blueprints/BP_FirstPersonGameMode.bSearchingAnomaly` (`self.GameModeRef`))))
    (set `/Game/FirstPerson/Blueprints/BP_FirstPersonGameMode.bSearchingAnomaly` true (`self.GameModeRef`))
    (set `self.RoomToSpawnAnomaly` (cast `/Game/ERooms` (`KismetMathLibrary.Conv_IntToByte` (`KismetMathLibrary.RandomIntegerInRange` 0 (- (enumcount `/Game/ERooms`) 1)))))
    (for _array_element (`self.RoomsRef`)
      (if (`|EnumEquality` (`/Game/Blueprints/BP_Room.RoomType` _array_element) (`self.RoomToSpawnAnomaly`))
        (set `/Game/Blueprints/BP_Room.bHasAnomaly` true _array_element)
        (bind _outactors (`GameplayStatics.GetAllActorsOfClass` "/Game/Blueprints/BP_MonsterSpawnPoint.BP_MonsterSpawnPoint_C"))
        (for _array_element_2 _outactors
          (if (`|EnumEquality` (`/Game/Blueprints/BP_MonsterSpawnPoint.Room` _array_element_2) (`self.RoomToSpawnAnomaly`))
            (`GameplayStatics.PlaySound2D` "/Game/Sounds/WHOOSH_Backstabber.WHOOSH_Backstabber" 1.0 1.0 0.0 null null)
            (`/Game/Blueprints/BP_MonsterSpawnPoint.VisibleThroughCam` _array_element_2)))))))

(fn `UserConstructionScript`)