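; BP_Phone is an actor that lets the player view security cameras in the current room through a phone interface.
; UsePhone toggles the view, gathering BP_SecurityCam actors matching the character's room, switching the view target to one and moving input from character to phone.
; It swaps the HUD for a WBP_Phone widget showing the camera count.
; Space cycles cameras, while E restores the player's view, input and HUD.
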(event `self.ReceiveBeginPlay`
  (bind _outactors (`GameplayStatics.GetAllActorsOfClass` "/Game/Blueprints/BP_SecurityCam.BP_SecurityCam_C"))
  (set `self.SecurityCamsRef` _outactors)
  (bind _asbp_first_person_character (cast `/Game/FirstPerson/Blueprints/BP_FirstPersonCharacter` (`GameplayStatics.GetPlayerCharacter` 0)))
  (set `self.CharacterRef` _asbp_first_person_character)
  (bind _returnvalue (`|CreateWidget` "/Game/Widgets/WBP_Phone.WBP_Phone_C"))
  (set `self.WidgetRef` _returnvalue))

(event `UsePhone`
  (bind _returnvalue (`GameplayStatics.GetPlayerController` 0))
  (bind _widgetref (`self.WidgetRef`))
  (`KismetArrayLibrary.Array_Clear` (`self.SecurityCamsRef`))
  (set `self.CamIndex` 0)
  (bind _outactors (`GameplayStatics.GetAllActorsOfClass` "/Game/Blueprints/BP_SecurityCam.BP_SecurityCam_C"))
  (for _array_element _outactors
    (if (`|EnumEquality` (`/Game/Blueprints/BP_SecurityCam.Room` _array_element) (`/Game/FirstPerson/Blueprints/BP_FirstPersonCharacter.CurrentRoom` (`self.CharacterRef`)))
      (`KismetArrayLibrary.Array_Add` (`self.SecurityCamsRef`) _array_element)))
  (if (`self.bIsCamOnline`)
    (`self.EndViewingCam`)
    (else
      (set `self.bIsCamOnline` true)
      (`self.DisableInput` (`GameplayStatics.GetPlayerCharacter` 0) _returnvalue)
      (`Controller.SetIgnoreLookInput` _returnvalue true)
      (`self.EnableInput` _returnvalue)
      (`self.ViewFromCam`)
      (`Widget.RemoveFromParent` (`/Game/FirstPerson/Blueprints/BP_FirstPersonCharacter.HUDRef` (`self.CharacterRef`)))
      (`/Game/Widgets/WBP_Phone.ChangeNbCams` _widgetref (`KismetArrayLibrary.Array_Length` (`self.SecurityCamsRef`)))
      (`UserWidget.AddToViewport` _widgetref 0)
      (set `PlayerController.bShowMouseCursor` true _returnvalue)
      (`WidgetBlueprintLibrary.SetInputMode_GameAndUIEx` _returnvalue null "DoNotLock" false))))

(event `EndViewingCam`
  (bind _returnvalue (`GameplayStatics.GetPlayerController` 0))
  (bind _returnvalue_2 (`GameplayStatics.GetPlayerCharacter` 0))
  (set `self.bIsCamOnline` false)
  (`self.DisableInput` _returnvalue)
  (`Controller.ResetIgnoreLookInput` _returnvalue)
  (`self.EnableInput` _returnvalue_2 _returnvalue)
  (`Widget.RemoveFromParent` (`self.WidgetRef`))
  (`PlayerController.SetViewTargetWithBlend` _returnvalue _returnvalue_2 0.0 "VTBlend_Linear" 0.0 false)
  (set `PlayerController.bShowMouseCursor` false _returnvalue)
  (`WidgetBlueprintLibrary.SetInputMode_GameOnly` _returnvalue)
  (`UserWidget.AddToViewport` (`/Game/FirstPerson/Blueprints/BP_FirstPersonCharacter.HUDRef` (`self.CharacterRef`)) 0))

(event `Key|SpaceBar`
  (params (Key :type "Key Structure"))
  (bind _returnvalue (+ (`self.CamIndex`) 1))
  (:`Pressed`
    (set `self.CamIndex` (select `bool` (> _returnvalue (- (`KismetArrayLibrary.Array_Length` (`self.SecurityCamsRef`)) 1)) :`false` _returnvalue))
    (`self.ViewFromCam`)))

(event `Key|E`
  (params (Key :type "Key Structure"))
  (:`Pressed`
    (`self.EndViewingCam`)))

(fn `UserConstructionScript`)

(fn `ViewFromCam`
  (`PlayerController.SetViewTargetWithBlend` (`GameplayStatics.GetPlayerController` 0) (`|GetArrayItem` (`self.SecurityCamsRef`) (`self.CamIndex`)) 0.0 "VTBlend_Linear" 0.0 false)
  (return))